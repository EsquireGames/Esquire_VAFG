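; Base Blueprint for interactive items in a pirate-themed game, highlighting the item mesh when an actor overlaps it.
; The construction script sizes the InteractableArea sphere from the mesh's bounding radius plus a configurable offset.
; Overlap begin enables the mesh's custom depth rendering if HighlightItem is set.
; The highlight is cleared on begin play, on overlap end, or on overlap begin when HighlightItem is off.
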(event `self.ReceiveBeginPlay`
  (`self.EndDisplayingHighlight`))

(event `self.ReceiveActorBeginOverlap`
  (params (OtherActor :type "Actor Object Reference"))
  (if (`self.HighlightItem?`)
    (`self.BeginDisplayingHighlight`)
    (else
      (`self.EndDisplayingHighlight` :!label _label))))

(event `self.ReceiveActorEndOverlap`
  (params (OtherActor :type "Actor Object Reference"))
  (goto _label))

(fn `BeginDisplayingHighlight`
  (`PrimitiveComponent.SetRenderCustomDepth` (`self.ItemMesh`) true))

(fn `EndDisplayingHighlight`
  (`PrimitiveComponent.SetRenderCustomDepth` (`self.ItemMesh`) false))

(fn `UserConstructionScript`
  (`SphereComponent.SetSphereRadius` (`self.InteractableArea`) (+ (`.SphereRadius` (`KismetSystemLibrary.GetComponentBounds` (`self.ItemMesh`))) (`self.ColliderOffsetFromStaticMesh`)) true))