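; VR startup pawn for the pirate game, with two motion controllers for highlighting and interacting with Pirate_BaseInteractiveItem actors.
; Controller hit boxes, sized from display mesh bounds plus an offset, toggle item highlights and grab flags on overlap.
; Right trigger sends InteractMessage to the first overlapped item; left trigger only prints debug text.
; Trigger releases clear widget pointer keys, but the branches choosing grab or widget press are unconnected.
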(event `self.ReceiveBeginPlay`
  (`self.EnableInput` (`GameplayStatics.GetPlayerController` 0)))

(event `self.ReceiveTick`
  (params (DeltaSeconds :type "Float (single-precision)")))

(event `InputAction|LeftTriggerAction`
  (params (Key :type "Key Structure"))
  (:`Pressed`
    (`KismetSystemLibrary.PrintString` "LeftGrab" true true (struct :`R` 1.0 :`G` 0.540281 :`B` 0.520381 :`A` 1.0) 0.5))
  (:`Released`
    (`self.StopPointerKeys`)))

(event `InputAction|RightTriggerAction`
  (params (Key :type "Key Structure"))
  (:`Pressed`
    (`KismetSystemLibrary.PrintString` "RightGrabGrab" true true (struct :`R` 1.0 :`G` 0.040931 :`B` 0.180734 :`A` 1.0) 0.5 :!label _label)
    (message `/Game/Blueprints/InteractiveItems/InteractableItemInterfaces.Interact` (`|GetArrayItem` (`PrimitiveComponent.GetOverlappingActors` (`self.R_MC_HitBox`) "/Game/Blueprints/InteractiveItems/Pirate_BaseInteractiveItem.Pirate_BaseInteractiveItem_C")) (`self.R_MotionController`)))
  (:`Released`
    (`self.StopPointerKeys`)))

(event `Key|MotionController_Right_Trigger`
  (params (Key :type "Key Structure"))
  (:`Pressed`
    (goto _label)))

(event `self.L_MC_HitBox.OnComponentBeginOverlap`
  (params (OverlappedComponent :type "PrimitiveComponent Object Reference") (OtherActor :type "Actor Object Reference") (OtherComp :type "PrimitiveComponent Object Reference") (OtherBodyIndex :type Integer) (bFromSweep :type Boolean) (SweepResult :type "HitResult Structure (by ref)"))
  ;[1 1 1] Manage Begin and End Overlaps on Left Motion Controller
  (bind _aspirate_base_interactive_item (cast `/Game/Blueprints/InteractiveItems/Pirate_BaseInteractiveItem` OtherActor))
  (`/Game/Blueprints/InteractiveItems/Pirate_BaseInteractiveItem.InteractiveHighlight` _aspirate_base_interactive_item)
  (set `self.L_MC_Hit?` true)
  (set `self.L_MC_CanGrab?` true)
  (set `self.CurrentInteractableObject` _aspirate_base_interactive_item))

(event `self.L_MC_HitBox.OnComponentEndOverlap`
  (params (OverlappedComponent :type "PrimitiveComponent Object Reference") (OtherActor :type "Actor Object Reference") (OtherComp :type "PrimitiveComponent Object Reference") (OtherBodyIndex :type Integer))
  ;[1 1 1] Manage Begin and End Overlaps on Left Motion Controller
  (set `self.L_MC_CanGrab?` false)
  (set `self.L_MC_Hit?` false)
  (bind _aspirate_base_interactive_item (cast `/Game/Blueprints/InteractiveItems/Pirate_BaseInteractiveItem` OtherActor))
  (message `/Game/Blueprints/InteractiveItems/InteractableItemInterfaces.StopHighlight` _aspirate_base_interactive_item))

(event `self.R_MC_HitBox.OnComponentBeginOverlap`
  (params (OverlappedComponent :type "PrimitiveComponent Object Reference") (OtherActor :type "Actor Object Reference") (OtherComp :type "PrimitiveComponent Object Reference") (OtherBodyIndex :type Integer) (bFromSweep :type Boolean) (SweepResult :type "HitResult Structure (by ref)"))
  ;[1 1 1] Manage Begin and End Overlaps on Right Motion Contoller
  (bind _aspirate_base_interactive_item (cast `/Game/Blueprints/InteractiveItems/Pirate_BaseInteractiveItem` OtherActor))
  (`/Game/Blueprints/InteractiveItems/Pirate_BaseInteractiveItem.InteractiveHighlight` _aspirate_base_interactive_item)
  (set `self.R_MC_Hit?` true)
  (set `self.R_MC_CanGrab?` true)
  (set `self.CurrentInteractableObject` _aspirate_base_interactive_item))

(event `self.R_MC_HitBox.OnComponentEndOverlap`
  (params (OverlappedComponent :type "PrimitiveComponent Object Reference") (OtherActor :type "Actor Object Reference") (OtherComp :type "PrimitiveComponent Object Reference") (OtherBodyIndex :type Integer))
  ;[1 1 1] Manage Begin and End Overlaps on Right Motion Contoller
  (bind _aspirate_base_interactive_item (cast `/Game/Blueprints/InteractiveItems/Pirate_BaseInteractiveItem` OtherActor))
  (message `/Game/Blueprints/InteractiveItems/InteractableItemInterfaces.StopHighlight` _aspirate_base_interactive_item)
  (set `self.R_MC_CanGrab?` false)
  (set `self.R_MC_Hit?` false))

(fn `EngagePointerKeys`
  (params (PrimaryInteractionWidget :type "WidgetInteractionComponent Object Reference") (SecondaryInteractionWidget :type "WidgetInteractionComponent Object Reference"))
  (bind _leftmousekeyreferance (`self.LeftMouseKeyReferance`))
  (`WidgetInteractionComponent.ReleasePointerKey` SecondaryInteractionWidget _leftmousekeyreferance)
  (`WidgetInteractionComponent.ReleasePointerKey` PrimaryInteractionWidget _leftmousekeyreferance)
  (`WidgetInteractionComponent.PressPointerKey` PrimaryInteractionWidget _leftmousekeyreferance))

(fn `HitBoxAdjuster`
  (params (`Motion Controller Component` :type "MotionControllerComponent Object Reference") (HitBoxToAdjust :type "BoxComponent Object Reference"))
  (bind (_returnvalue_origin _returnvalue_boxextent) (`KismetMathLibrary.BreakBoxSphereBounds` (`StaticMesh.GetBounds` (`MotionControllerComponent.CustomDisplayMesh` `Motion Controller Component`))))
  (`BoxComponent.SetBoxExtent` HitBoxToAdjust (+ _returnvalue_boxextent (`self.MC_CollisionOffset`)) true))

(fn `StopPointerKeys`
  (`WidgetInteractionComponent.ReleasePointerKey` (`self.L_WidgetInteraction`) (`self.LeftMouseKeyReferance`))
  (`WidgetInteractionComponent.ReleasePointerKey` (`self.R_WidgetInteraction`) (`self.LeftMouseKeyReferance`)))

(fn `UserConstructionScript`
  (`self.HitBoxAdjuster` (`self.L_MotionController`) (`self.L_MC_HitBox`))
  (`self.HitBoxAdjuster` (`self.R_MotionController`) (`self.R_MC_HitBox`)))